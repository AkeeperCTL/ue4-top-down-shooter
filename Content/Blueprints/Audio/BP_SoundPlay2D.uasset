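; BP_SoundPlay2D is a placeable helper that plays a non-spatial 2D sound, flagged as non-UI, when play begins.
; Its Audio2D component supplies the sound asset, and the construction script stops that component.
; BeginPlay checks PlayOnBeginPlay, then calls PlaySound2D with that asset and the volume, pitch and start-time variables instead of playing the component itself.
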(event EventBeginPlay
  (if (Variables|SoundPlaySettings|GetPlayOnBeginPlay)
    (Audio|PlaySound2D (Variables|/Script/Engine.AudioComponent|GetSound (Variables|Default|GetAudio2D)) (Variables|SoundPlaySettings|GetVolume%20Multiplier) (Variables|SoundPlaySettings|GetPitch%20Multiplier) (Variables|SoundPlaySettings|GetStart%20Time) 0 0 false)))

(event Collision|EventActorBeginOverlap
  (params (OtherActor :type Actor%20Object%20Reference)))

(event EventTick
  (params (DeltaSeconds :type Float%20%28single-precision%29)))

(fn ConstructionScript
  (Audio|Components|Audio|Stop (Variables|Default|GetAudio2D)))