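; Procedural arena actor that builds a tiled floor ringed by walls and doors on BeginPlay, then populates it by arena type.
; Doors are placed at eligible intervals using seeded, count-weighted rolls, and each wall gets an indexed collision actor for later removal.
; Start and Checkpoint arenas get a shop, Boss a coliseum, and Enemy houses fitted by box traces.
; Teardown, also run from the construction script, clears tracked pieces and sweeps owned actors by class.
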(event Custom|OnArenaGenerated
  (bind (_returnvalue_roll _returnvalue_pitch _returnvalue) (Utilities|Arena:GetFirstDoorReverseDirection))
  (bind (_returnvalue_roll_2 _returnvalue_pitch_2 _returnvalue_2) (Utilities|Arena:GetFirstDoorReverseDirection))
  ;[1 1 1] Создание продавца или колизея босса или прочего
  (Variables|ArenaGeneration|SetIsGenerationComplete true)
  (switch Utilities|FlowControl|Switch|SwitchonE_Arena_Types (Variables|ArenaGeneration|GetArenaType)
    (:NewEnumerator0
      ;;[1 1 1] СПАВН ТОРГОВЦА
      (bind _floormesh (Floor|GetFloorCenterInstance :!label _label))
      (bind _returnvalue_3 (Game|SpawnActorfromClass "/Game/Blueprints/Arena/ProceduralActors/BP_Shop.BP_Shop_C" (Math|Transform|MakeTransform (Transformation|GetWorldLocation _floormesh) (Math|Rotator|MakeRotator _returnvalue_roll_2 _returnvalue_pitch_2 _returnvalue_2)) "AlwaysSpawn" self 0))
      (Variables|OtherActors|SetArenaShop _returnvalue_3))
    (:NewEnumerator1
      ;;[1 1 1] СПАВН ДОМОВ
      (CreateMeshes|CreateHouses) ; СПАВН ДОМОВ
    )
    (:NewEnumerator2
      (goto _label))
    (:NewEnumerator3
      ;;[1 1 1] СПАВН БОССА
      (bind _floormesh_2 (Floor|GetFloorCenterInstance))
      (bind _returnvalue_4 (Game|SpawnActorfromClass "/Game/Blueprints/Arena/ProceduralActors/BP_BossColiseum.BP_BossColiseum_C" (Math|Transform|MakeTransform (Transformation|GetWorldLocation _floormesh_2) (Math|Rotator|MakeRotator _returnvalue_roll _returnvalue_pitch _returnvalue)) "AlwaysSpawn" self 0))
      (Variables|OtherActors|SetArenaBossColiseum _returnvalue_4))))

(event Custom|OnArenaDestroyed
  ;[1 1 1] Событие после уничтожения арены
  (Variables|ArenaGeneration|SetIsGenerationComplete false))

(event EventBeginPlay
  (if (not (Variables|ArenaGeneration|GetIsGenerationComplete))
    (ArenaGeneration|GenerateNewArena)))

(event Collision|EventActorBeginOverlap
  (params (OtherActor :type Actor%20Object%20Reference)))

(event EventTick
  (params (DeltaSeconds :type Float%20%28single-precision%29)))

(event EventOnWallCollisionDeleted
  (params (WallIndex :type Integer))
  (bind _spawnedwalls (Variables|Walls&FloorCreation|GetSpawnedWalls))
  (bind _returnvalue (Utilities|Array|LastIndex _spawnedwalls))
  ;[1 1 1] Событие при уничтожении коллизии стены
  (Components|DestroyComponent (Utilities|Array|Get(acopy) _spawnedwalls WallIndex))
  (Utilities|Array|SetArrayElem _spawnedwalls WallIndex (Utilities|Array|Get(acopy) _spawnedwalls _returnvalue) true)
  (Utilities|Array|RemoveIndex (Variables|Walls&FloorCreation|GetSpawnedWalls) _returnvalue))

(event EventDestroyed
  (ArenaGeneration|DestroyCurrentArena))

(fn ConstructionScript
  (ArenaGeneration|DestroyCurrentArena))

(fn CreateWallCopies
  (params (TileX :type Integer) (Tile%20Y :type Integer) (Tile%20Step :type Float%20%28single-precision%29))
  (bind _wallsamplepoint (Variables|Default|GetWallSamplePoint))
  (bind _relativelocation (Variables|/Script/Engine.SceneComponent|GetRelativeLocation _wallsamplepoint))
  (LocalVariables|SetLocalTileX (- TileX 1))
  (bind _output_get (LocalVariables|SetLocalTileY (- Tile%20Y 1)))
  (bind _output_get_2 (LocalVariables|SetLocalTileStep Tile%20Step))
  ;[1 1 1] НИЖНИЕ СТЕНЫ
  (for _index (range 0 _output_get)
    (if (or (Utilities|Enum|Equal(Enum) (Variables|ArenaGeneration|GetArenaType) "NewEnumerator0") (!= _index 0))
      (CreateMeshes|SpawnDoororWall (== (Math|Integer|%(Integer) _index (Variables|ArenaDoorGeneration|GetDoorDesiredIndex)) (Variables|ArenaDoorGeneration|GetDoorDesiredRemainder)) (Math|Vector|MakeVector (.x _relativelocation) (* _index _output_get_2) (.z _relativelocation)) "0,90.000000, 0" (.BottomCount (Utilities|Struct|BreakF_ArenaDoor_Count_Info (Variables|ArenaDoorGeneration|GetDoorCountInfo)))))
    ;[1 1 1] ВЕРХНИЕ СТЕНЫ
    (CreateMeshes|SpawnDoororWall (== (Math|Integer|%(Integer) _index (Variables|ArenaDoorGeneration|GetDoorDesiredIndex)) (Variables|ArenaDoorGeneration|GetDoorDesiredRemainder)) (Math|Vector|MakeVector (+ (* (LocalVariables|GetLocalTileX) (LocalVariables|GetLocalTileStep)) (/ (LocalVariables|GetLocalTileStep) 2.0)) (* _index (LocalVariables|GetLocalTileStep)) (.z (Variables|/Script/Engine.SceneComponent|GetRelativeLocation (Variables|Default|GetWallSamplePoint)))) "0.0,-90.000000,0.0" (.TopCount (Utilities|Struct|BreakF_ArenaDoor_Count_Info (Variables|ArenaDoorGeneration|GetDoorCountInfo)))))
  ;[1 1 1] СТЕНЫ СЛЕВА
  (for _index_2 (range 0 (LocalVariables|GetLocalTileX))
    (CreateMeshes|SpawnDoororWall (== (Math|Integer|%(Integer) _index_2 (Variables|ArenaDoorGeneration|GetDoorDesiredIndex)) (Variables|ArenaDoorGeneration|GetDoorDesiredRemainder)) (Math|Vector|MakeVector (* _index_2 (LocalVariables|GetLocalTileStep)) (- 0.0 (/ (LocalVariables|GetLocalTileStep) 2.0)) (.z (Variables|/Script/Engine.SceneComponent|GetRelativeLocation (Variables|Default|GetWallSamplePoint)))) "0.0,180.000000,0.000000" (.LeftCount (Utilities|Struct|BreakF_ArenaDoor_Count_Info (Variables|ArenaDoorGeneration|GetDoorCountInfo))))
    ;[1 1 1] СТЕНЫ СПРАВА
    (CreateMeshes|SpawnDoororWall (== (Math|Integer|%(Integer) _index_2 (Variables|ArenaDoorGeneration|GetDoorDesiredIndex)) (Variables|ArenaDoorGeneration|GetDoorDesiredRemainder)) (Math|Vector|MakeVector (* _index_2 (LocalVariables|GetLocalTileStep)) (+ (* (LocalVariables|GetLocalTileY) (LocalVariables|GetLocalTileStep)) (/ (LocalVariables|GetLocalTileStep) 2.0)) (.z (Variables|/Script/Engine.SceneComponent|GetRelativeLocation (Variables|Default|GetWallSamplePoint)))) "0, 0, 0" (.RightCount (Utilities|Struct|BreakF_ArenaDoor_Count_Info (Variables|ArenaDoorGeneration|GetDoorCountInfo))))))

(fn CreateFloorCopies
  (params (TileX :type Integer) (TileY :type Integer) (TileStep :type Float%20%28single-precision%29))
  (for _index (range 0 (- TileX 1))
    (for _index_2 (range 0 (- TileY 1))
      (bind _returnvalue (AddComponent|AddStaticMeshComponent false (Math|Transform|MakeTransform (Math|Vector|MakeVector (* _index TileStep) (* _index_2 TileStep) 0.0))))
      (Utilities|Map|Add (Variables|Walls&FloorCreation|GetFloorMatrixOrderMap) (Math|Vector2D|MakeVector2D (+ (Math|Conversions|ToFloat(Integer) _index) 1.0) (+ (Math|Conversions|ToFloat(Integer) _index_2) 1.0)) _returnvalue))))

(fn SpawnDoororWall
  (params (CanBeDoor? :type Boolean) (RelativeTransform :type Vector) (RelativeRotation :type Rotator) (DesiredDoorCount :type Integer))
  (bind _returnvalue (Transformation|GetActorTransform))
  (bind _returnvalue_2 (Math|Transform|TransformLocation _returnvalue RelativeTransform))
  (bind _returnvalue_3 (Math|Transform|TransformRotation _returnvalue RelativeRotation))
  (bind (_roll _pitch _yaw) (Math|Rotator|BreakRotator _returnvalue_3))
  (bind _returnvalue_4 (+ _yaw 9e+01))
  (bind _returnvalue_5 (Math|Rotator|MakeRotator _roll _pitch _returnvalue_4))
  (bind _output_get (LocalVariables|SetLocal%20Door%20Count DesiredDoorCount))
  ;[1 1 1] Фикс предупреждения / на 0 при генерации арены
  (if (!= _output_get 0)
    (if (and CanBeDoor? (Class|KismetMathLibrary|RandomBoolwithWeightfromStream (/ (Math|Conversions|ToFloat(Integer) (- (LocalVariables|GetLocal%20Door%20Count) (Utilities|Array|Length (Variables|ArenaDoorGeneration|GetSpawnedDoors)))) (Math|Conversions|ToFloat(Integer) (LocalVariables|GetLocal%20Door%20Count))) (Variables|ArenaGeneration|GetRandomStreamVar)))
      ;[1 1 1] СОЗДАТЬ ДВЕРЬ
      (bind _returnvalue_6 (Game|SpawnActorfromClass (Variables|ArenaGeneration|GetUsedDoorClass) (Math|Transform|MakeTransform _returnvalue_2 _returnvalue_5 "1,1,1") "AlwaysSpawn" self 0))
      (Utilities|Array|Add (Variables|ArenaDoorGeneration|GetSpawnedDoors) _returnvalue_6)
      (else
        ;[1 1 1] СОЗДАТЬ ОБЫЧНУЮ СТЕНУ
        (bind _returnvalue_7 (AddComponent|AddStaticMeshComponent false (Math|Transform|MakeTransform RelativeTransform RelativeRotation "1,1,1") :!label _label))
        (Components|StaticMesh|SetStaticMesh _returnvalue_7 (.OutItem (Utilities|Array|Random (Variables|ArenaGeneration|GetUsedWallRandomMeshes))))
        (bind _returnvalue_8 (Utilities|Array|Add (Variables|Walls&FloorCreation|GetSpawnedWalls) _returnvalue_7))
        ;;[1 1 1] Создать номер стены
        (bind _returnvalue_9 (Game|SpawnActorfromClass (Variables|ArenaGeneration|GetUsedWallCollisionClass) (Math|Transform|MakeTransform _returnvalue_2 _returnvalue_5 "1,1,1") "AlwaysSpawn" self 0))
        (Class|BPIArenaListener|OnWallCollisionGenerated(Message) _returnvalue_9 _returnvalue_8 self)
        (Utilities|Array|AddUnique (Variables|Walls&FloorCreation|GetSpawnedWallCollisions) _returnvalue_9)))
    (else
      (goto _label))))

(fn CreateHouses
  (bind _randomstreamvar (Variables|ArenaGeneration|GetRandomStreamVar))
  (bind _arenatilesx (Variables|ArenaGeneration|GetArenaTilesX))
  (bind _arenatilesy (Variables|ArenaGeneration|GetArenaTilesY))
  (bind _returnvalue (Math|Random|RandomIntegerinRangefromStream 0 1 _randomstreamvar))
  (bind _returnvalue_2 (Math|Conversions|ToBoolean(Integer) _returnvalue))
  (LocalVariables|SetLocalFloorSquare (* (Variables|ArenaGeneration|GetArenaTilesX) (Variables|ArenaGeneration|GetArenaTilesY)))
  (if (>= (LocalVariables|GetLocalFloorSquare) 9)
    ;[1 1 1] Обработка исключения 3х3
    (if (== (LocalVariables|GetLocalFloorSquare) 9)
      (bind _floormesh (Floor|GetFloorCenterInstance))
      (Utilities|IsValid _floormesh
        (:Is%20Valid
          (bind _returnvalue_3 (Game|SpawnActorfromClass "/Game/Blueprints/Arena/ProceduralActors/BP_House1x1.BP_House1x1_C" (Math|Transform|MakeTransform (Transformation|GetWorldLocation _floormesh) (Math|Rotator|MakeRotator 0.0 0.0 (Math|Float|SelectFloat -9e+01 0.0 (Utilities|Enum|Equal(Enum) "" "X")))) "AlwaysSpawn" 0 0))
          (Utilities|Array|AddUnique (Variables|OtherActors|GetSpawnedHouses) _returnvalue_3))))
    (bind _output_get (LocalVariables|SetLocalInitialHouseSize "NewEnumerator3"))
    (bind (_x_size _y_size) (Houses|GetIntSizefromEnum _output_get))
    (LocalVariables|SetLocalCurrentHouseXSize _x_size)
    (LocalVariables|SetLocalCurrentHouseYSize _y_size)
    (for _index (range 1 _arenatilesx)
      (if true
        (for _index_2 (range 1 _arenatilesy)
          (bind _floormesh_2 (Floor|GetFloorInstance (Math|Vector2D|MakeVector2D (Math|Conversions|ToFloat(Integer) _index) (Math|Conversions|ToFloat(Integer) _index_2))))
          (if (== (Math|Integer|%(Integer) _index_2 (+ (LocalVariables|GetLocalCurrentHouseYSize) (Math|Integer|SelectInt 1 0 (and (< _index_2 (/ _arenatilesy 2)) (< _index (/ _arenatilesx 2)))))) 0)
            (bind _can (Houses|CanSpawnHouseatFloorNew _floormesh_2 (Utilities|Enum|ByteToEnumE_House_Sizes (LocalVariables|GetLocalInitialHouseSize))))
            (if _can
              (bind _house_class (Houses|GetActorClassfromSizeEnum (LocalVariables|GetLocalInitialHouseSize)))
              (bind _returnvalue_4 (Game|SpawnActorfromClass _house_class (Math|Transform|MakeTransform (Transformation|GetWorldLocation _floormesh_2) (Math|Rotator|MakeRotator 0.0 0.0 (Math|Float|SelectFloat (Math|Float|SelectFloat -9e+01 0.0 _returnvalue_2) (Math|Float|SelectFloat 9e+01 0.0 _returnvalue_2) (Math|Conversions|ToBoolean(Integer) (Math|Random|RandomIntegerinRangefromStream 0 1 _randomstreamvar))))) "AlwaysSpawn" self 0))
              (Utilities|Array|AddUnique (Variables|OtherActors|GetSpawnedHouses) _returnvalue_4)
              ;[1 1 1] СЛУЧАЙНЫЙ ВЫБОР ЗДАНИЯ ПЕРЕД СЛЕДУЮЩИМ СПАВНОМ
              (bind _output_get_2 (LocalVariables|SetLocalInitialHouseSize (Utilities|Select :Index (Math|Random|RandomIntegerinRangefromStream 0 3 (Variables|ArenaGeneration|GetRandomStreamVar)) :Option%200 "NewEnumerator3" :Option%201 "NewEnumerator2" :Option%202 "NewEnumerator1" :Option%203 "NewEnumerator0")))
              (bind (_x_size_2 _y_size_2) (Houses|GetIntSizefromEnum _output_get_2))
              (LocalVariables|SetLocalCurrentHouseXSize _x_size_2)
              (LocalVariables|SetLocalCurrentHouseYSize _y_size_2))))))
    (else
      (Development|PrintString "Арена: Площадь арены слишком мала (<9), чтобы спавнить постройки" true true "(R=1.000000,G=0.000000,B=0.009844,A=1.000000)" 5.0))))

(fn GenerateNewArena
  ;[1 1 1] ОЧИЩЕНИЕ ПОСТРОЕННЫХ КОМПОНЕНТОВ.
  ;
  ; КОГДА В РЕДАКТОРЕ ВЫЗЫВАЕШЬ ГЕНЕРАЦИЮ АРЕНЫ, ТО СТАРАЯ АРЕНА НЕ ИСЧЕЗАЕТ
  (ArenaGeneration|DestroyCurrentArena)
  (CreateMeshes|CreateFloorCopies (Variables|ArenaGeneration|GetArenaTilesX) (Variables|ArenaGeneration|GetArenaTilesY) (Variables|ArenaGeneration|GetArenaTilesStep))
  (CreateMeshes|CreateWallCopies (Variables|ArenaGeneration|GetArenaTilesX) (Variables|ArenaGeneration|GetArenaTilesY) (Variables|ArenaGeneration|GetArenaTilesStep))
  (CallFunction|OnArenaGenerated))

(fn DestroyCurrentArena
  (bind _floormatrixordermap (Variables|Walls&FloorCreation|GetFloorMatrixOrderMap))
  (bind _arenashop (Variables|OtherActors|GetArenaShop))
  (bind _spawnedwallcollisions (Variables|Walls&FloorCreation|GetSpawnedWallCollisions))
  (bind _arenabosscoliseum (Variables|OtherActors|GetArenaBossColiseum))
  (bind _spawneddoors (Variables|ArenaDoorGeneration|GetSpawnedDoors))
  (bind _spawnedhouses (Variables|OtherActors|GetSpawnedHouses))
  (bind _spawnedwalls (Variables|Walls&FloorCreation|GetSpawnedWalls))
  ;[1 1 1] УДАЛЕНИЕ ПРОЧИХ АКТЁРОВ
  (Utilities|IsValid _arenashop
    (:Is%20Valid
      (Actor|DestroyActor _arenashop))
    (:Is%20Not%20Valid
      _))
  (Utilities|IsValid _arenabosscoliseum
    (:Is%20Valid
      (Actor|DestroyActor _arenabosscoliseum))
    (:Is%20Not%20Valid
      _))
  ;[1 1 1] УНИЧТОЖЕНИЕ ДОМОВ
  (for _array_element _spawnedhouses
    (Utilities|IsValid _array_element
      (:Is%20Valid
        (Actor|DestroyActor _array_element))))
  (Utilities|Array|Clear _spawnedhouses)
  (Utilities|Arena:RemoveActorsbyClass "/Game/Blueprints/Arena/BP_ProceduralCreatedBuildingsAbstract.BP_ProceduralCreatedBuildingsAbstract_C"
    (:Completed
      ;[1 1 1] УНИЧТОЖЕНИЕ СТЕН
      (for _array_element_2 _spawnedwalls
        (Utilities|IsValid _array_element_2
          (:Is%20Valid
            (Components|DestroyComponent _array_element_2))))
      (Utilities|Array|Clear _spawnedwalls)
      ;[1 1 1] УНИЧТОЖЕНИЕ НОМЕРАЦИИ СТЕН
      (for _array_element_3 _spawnedwallcollisions
        (Utilities|IsValid _array_element_3
          (:Is%20Valid
            (Actor|DestroyActor _array_element_3))))
      (Utilities|Array|Clear _spawnedwallcollisions)
      (Utilities|Arena:RemoveActorsbyClass (Variables|ArenaGeneration|GetUsedWallCollisionClass)
        (:Completed
          ;[1 1 1] УНИЧТОЖЕНИЕ ПОЛА
          (bind _values (Utilities|Map|Values _floormatrixordermap))
          (for _array_element_4 _values
            (Utilities|IsValid _array_element_4
              (:Is%20Valid
                (Components|DestroyComponent _array_element_4))))
          (Utilities|Map|Clear _floormatrixordermap)
          ;[1 1 1] УНИЧТОЖЕНИЕ ДВЕРЕЙ
          (for _array_element_5 _spawneddoors
            (Utilities|IsValid _array_element_5
              (:Is%20Valid
                (Actor|DestroyActor _array_element_5))))
          (Utilities|Array|Clear _spawneddoors)
          (Utilities|Arena:RemoveActorsbyClass (Variables|ArenaGeneration|GetUsedDoorClass)
            (:Completed
              (CallFunction|OnArenaDestroyed)
              (return))))))))

(fn GetFloorInstance
  (params (Vector :type Vector%202D%20Structure :default "(X=1.000000,Y=1.000000)"))
  (bind _floormatrixordermap (Variables|Walls&FloorCreation|GetFloorMatrixOrderMap))
  (bind (_value _returnvalue) (Utilities|Map|Find _floormatrixordermap Vector))
  (if _returnvalue
    (return _value)
    (else
      (Development|PrintString "Arena: Can't find the floor instance by input vector" true true "(R=1.000000,G=0.000000,B=0.000000,A=1.000000)" 5.0))))

(fn GetFloorCenterInstance
  (bind _floormesh (Floor|GetFloorInstance (Math|Vector2D|MakeVector2D (Math|Conversions|ToFloat(Integer) (Math|Float|Round (+ (/ (Math|Conversions|ToFloat(Integer) (Variables|ArenaGeneration|GetArenaTilesX)) 2.0) 0.1))) (Math|Conversions|ToFloat(Integer) (Math|Float|Round (+ (/ (Math|Conversions|ToFloat(Integer) (Variables|ArenaGeneration|GetArenaTilesY)) 2.0) 0.1))))))
  (return _floormesh))

(fn GetLargestAxis
  (bind _arenatilesx (Variables|ArenaGeneration|GetArenaTilesX))
  (bind _arenatilesy (Variables|ArenaGeneration|GetArenaTilesY))
  (if (== _arenatilesx _arenatilesy)
    (return "ALL")
    (else
      (return (Utilities|String|SelectString "X" "Y" (> _arenatilesx _arenatilesy))))))

(fn GetActorClassfromSizeEnum
  (params (HouseSize :type E_House_Sizes%20Enum :default "NewEnumerator0"))
  (switch Utilities|FlowControl|Switch|SwitchonE_House_Sizes HouseSize
    (:NewEnumerator3
      (LocalVariables|SetSelectedClass "/Game/Blueprints/Arena/ProceduralActors/BP_House2x2.BP_House2x2_C"))
    (:NewEnumerator2
      (LocalVariables|SetSelectedClass "/Game/Blueprints/Arena/ProceduralActors/BP_House1x3.BP_House1x3_C"))
    (:NewEnumerator1
      (LocalVariables|SetSelectedClass "/Game/Blueprints/Arena/ProceduralActors/BP_House1x2.BP_House1x2_C"))
    (:NewEnumerator0
      (LocalVariables|SetSelectedClass "/Game/Blueprints/Arena/ProceduralActors/BP_House1x1.BP_House1x1_C")))
  (return (LocalVariables|GetSelectedClass)))

(fn GetIntSizefromEnum
  (params (House%20Size :type E_House_Sizes%20Enum :default "NewEnumerator3"))
  (Utilities|FlowControl|Sequence
    (:then_0
      (switch Utilities|FlowControl|Switch|SwitchonE_House_Sizes House%20Size
        (:NewEnumerator3
          (LocalVariables|SetCurrentY 2))
        (:NewEnumerator2
          (LocalVariables|SetCurrentY 3))
        (:NewEnumerator1
          (LocalVariables|SetCurrentY 2))
        (:NewEnumerator0
          (LocalVariables|SetCurrentY 1))))
    (:then_1
      (switch Utilities|FlowControl|Switch|SwitchonE_House_Sizes House%20Size
        (:NewEnumerator3
          (LocalVariables|SetCurrentX 2))
        (:NewEnumerator2
          (LocalVariables|SetCurrentX 1 :!label _label))
        (:NewEnumerator1
          (goto _label))
        (:NewEnumerator0
          (goto _label)))))
  (return (LocalVariables|GetCurrentX) (LocalVariables|GetCurrentY)))

(fn CanSpawnHouseatFloor
  (params (FloorComponent :type Scene%20Component%20Object%20Reference) (InitialHouseSize :type E_House_Sizes%20Enum :default "NewEnumerator3") (InitialLargestAxis :type String))
  (bind _arenatilesstep (Variables|ArenaGeneration|GetArenaTilesStep))
  (bind _arenatilesstep_2 (Variables|ArenaGeneration|GetArenaTilesStep))
  (bind _arenatilesstep_3 (Variables|ArenaGeneration|GetArenaTilesStep))
  (bind _returnvalue (/ _arenatilesstep_2 2.5))
  (bind _returnvalue_2 (/ _arenatilesstep_3 2.5))
  (bind _returnvalue_3 (+ _returnvalue 2e+02))
  (bind _returnvalue_4 (+ _returnvalue_2 2e+02))
  (LocalVariables|SetLocalFloorComponent FloorComponent)
  (LocalVariables|SetLocalHouseSizeEnum InitialHouseSize)
  (LocalVariables|SetLocalLargestAxis InitialLargestAxis)
  (Utilities|FlowControl|ForLoopwithBreak (Math|Conversions|ToInteger(Byte) (LocalVariables|GetLocalHouseSizeEnum)) (|GetNumEnumEntries) :!label _label
    (:LoopBody
      (bind (_x_size _y_size) (Houses|GetIntSizefromEnum (LocalVariables|GetLocalHouseSizeEnum)))
      (LocalVariables|SetLocalHouseXSize (Math|Integer|SelectInt _x_size _y_size (or (Utilities|Enum|Equal(Enum) (LocalVariables|GetLocalLargestAxis) "Y") (Utilities|Enum|Equal(Enum) (LocalVariables|GetLocalLargestAxis) "ALL"))))
      (LocalVariables|SetLocalHouseYSize (Math|Integer|SelectInt _y_size _x_size (or (Utilities|Enum|Equal(Enum) (LocalVariables|GetLocalLargestAxis) "Y") (Utilities|Enum|Equal(Enum) (LocalVariables|GetLocalLargestAxis) "ALL"))))
      (if (and (Utilities|Enum|Equal(Enum) (LocalVariables|GetLocalLargestAxis) "Y") (Utilities|Enum|Equal(Enum) (LocalVariables|GetLocalLargestAxis) "ALL"))
        (Development|PrintString "ОБРАБОТКА Х")
        (return false (LocalVariables|GetLocalHouseSizeEnum) "")
        (else
          ;[1 1 1] Трейс по Х настолько, насколько длинный по Х дом
          (bind _returnvalue_5 (Collision|BoxTraceByChannel (+ (Transformation|GetWorldLocation (LocalVariables|GetLocalFloorComponent)) (Math|Vector|MakeVector (* _arenatilesstep -1.0) 0.0 _returnvalue_3)) (+ (Transformation|GetWorldLocation (LocalVariables|GetLocalFloorComponent)) (Math|Vector|MakeVector (* (+ (LocalVariables|GetLocalHouseXSize) 1) _arenatilesstep) 0.0 _returnvalue_3)) (Math|Vector|MakeVector _returnvalue _returnvalue _returnvalue) "0, 0, 0" "TraceTypeQuery1" true 0 "ForDuration" false "(R=1.000000,G=0.000000,B=0.000000,A=1.000000)" "(R=1.000000,G=0.771456,B=0.000000,A=1.000000)"))
          ;;[1 1 1] Если нет препятствий
          (if (not _returnvalue_5)
            ;[1 1 1] Трейс по У настолько, насколько длинный по У дом
            (bind _returnvalue_6 (Collision|BoxTraceByChannel (+ (Transformation|GetWorldLocation (LocalVariables|GetLocalFloorComponent)) (Math|Vector|MakeVector 0.0 0.0 _returnvalue_4)) (+ (Transformation|GetWorldLocation (LocalVariables|GetLocalFloorComponent)) (Math|Vector|MakeVector 0.0 (* (LocalVariables|GetLocalHouseYSize) (Variables|ArenaGeneration|GetArenaTilesStep)) _returnvalue_4)) (Math|Vector|MakeVector _returnvalue_2 _returnvalue_2 _returnvalue_2) "0, 0, 0" "TraceTypeQuery1" true 0 "None" false "(R=0.000000,G=1.000000,B=0.006319,A=1.000000)" "(R=1.000000,G=0.958267,B=0.000000,A=1.000000)"))
            ;;[1 1 1] Если не препятствий
            (if (not _returnvalue_6)
              (LocalVariables|SetLocalCanSpawnInRecurse? true)
              (goto _label Break)
              (else
                (LocalVariables|SetLocalCanSpawnInRecurse? false)))
            (else
              (LocalVariables|SetLocalCanSpawnInRecurse? false)
              (if (< (LocalVariables|GetLocalHouseSizeEnum) (Math|Conversions|ToByte(Integer) (- (|GetNumEnumEntries) 1)))
                (LocalVariables|SetLocalHouseSizeEnum (Utilities|Enum|ByteToEnumE_House_Sizes (+ (LocalVariables|GetLocalHouseSizeEnum) 1)))
                (Development|PrintString (Utilities|String|Append "Пробую дом другого размера = " (Utilities|String|EnumtoString (LocalVariables|GetLocalHouseSizeEnum)) " Ось: " (LocalVariables|GetLocalLargestAxis)) true true "(R=1.000000,G=0.000000,B=0.049179,A=1.000000)" 5.0)))))))
    (:Completed
      (if (LocalVariables|GetLocalCanSpawnInRecurse?)
        (return true (LocalVariables|GetLocalHouseSizeEnum) "")
        (elif (Utilities|Enum|NotEqual(Enum) (LocalVariables|GetLocalLargestAxis) "X")
          (LocalVariables|SetLocalLargestAxis "X")
          (goto _label)
          (else
            (return false (LocalVariables|GetLocalHouseSizeEnum) "")))))))

(fn CanSpawnHouseatFloorNew
  (params (FloorComponent :type Scene%20Component%20Object%20Reference) (InitialHouseSize :type E_House_Sizes%20Enum :default "NewEnumerator3"))
  (bind _arenatilesstep (Variables|ArenaGeneration|GetArenaTilesStep))
  (bind _arenatilesstep_2 (Variables|ArenaGeneration|GetArenaTilesStep))
  (bind _arenatilesstep_3 (Variables|ArenaGeneration|GetArenaTilesStep))
  (bind _returnvalue (/ _arenatilesstep_2 2.5))
  (bind _returnvalue_2 (/ _arenatilesstep_3 2.5))
  (bind _returnvalue_3 (+ _returnvalue 2e+02))
  (bind _returnvalue_4 (+ _returnvalue_2 2e+02))
  (LocalVariables|SetLocalFloorComponent FloorComponent)
  (bind _output_get (LocalVariables|SetLocalHouseSizeEnum InitialHouseSize))
  (bind (_x_size _y_size) (Houses|GetIntSizefromEnum _output_get))
  (LocalVariables|SetLocalHouseXSize _x_size)
  (LocalVariables|SetLocalHouseYSize _y_size)
  ;[1 1 1] Трейс по Х настолько, насколько длинный по Х дом
  (bind _returnvalue_5 (Collision|BoxTraceByChannel (+ (Transformation|GetWorldLocation (LocalVariables|GetLocalFloorComponent)) (Math|Vector|MakeVector (* _arenatilesstep -1.0) 0.0 _returnvalue_3)) (+ (Transformation|GetWorldLocation (LocalVariables|GetLocalFloorComponent)) (Math|Vector|MakeVector (* (+ (LocalVariables|GetLocalHouseXSize) 1) _arenatilesstep) 0.0 _returnvalue_3)) (Math|Vector|MakeVector _returnvalue _returnvalue _returnvalue) "0, 0, 0" "TraceTypeQuery1" false 0 "ForDuration" false "(R=1.000000,G=0.000000,B=0.000000,A=1.000000)" "(R=1.000000,G=0.771456,B=0.000000,A=1.000000)"))
  ;;[1 1 1] Если нет препятствий
  (if (not _returnvalue_5)
    ;[1 1 1] Трейс по У настолько, насколько длинный по У дом
    (bind _returnvalue_6 (Collision|BoxTraceByChannel (+ (Transformation|GetWorldLocation (LocalVariables|GetLocalFloorComponent)) (Math|Vector|MakeVector 0.0 0.0 _returnvalue_4)) (+ (Transformation|GetWorldLocation (LocalVariables|GetLocalFloorComponent)) (Math|Vector|MakeVector 0.0 (* (LocalVariables|GetLocalHouseYSize) (Variables|ArenaGeneration|GetArenaTilesStep)) _returnvalue_4)) (Math|Vector|MakeVector _returnvalue_2 _returnvalue_2 _returnvalue_2) "0, 0, 0" "TraceTypeQuery1" false 0 "ForDuration" false "(R=0.000000,G=1.000000,B=0.006319,A=1.000000)" "(R=1.000000,G=0.958267,B=0.000000,A=1.000000)"))
    ;;[1 1 1] Если не препятствий
    (if (not _returnvalue_6)
      (return true)
      (else
        _)))
  (return false))