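; Top-down shooter player character that maps input to sprint, walk and aim movement states, hip or ironsight fire montages, and interaction.
; Zoom input sets a clamped target camera boom length, which Tick interpolates toward.
; Tick also passes stamina to the C++ parent, sets sprint-based consumption, and prints debug info.
; A per-frame cursor trace caches the actor and distance for range-checked BPI_Interactable calls.
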(event EventBeginPlay
  (Camera|SetupCameraDesiredHeight))

(event EventTick
  (params (DeltaSeconds :type Float%20%28single-precision%29))
  ;[1 1 1 1 24] ОБНОВЛЕНИЕ КАДРА
  (Utilities|FlowControl|Sequence
    (:then_0
      (HealthAndStamina|UpdateStamina))
    (:then_1
      (Debug|DebugDrawInfo))
    (:then_2
      (Camera|InterpolateCamera (Utilities|Time|GetWorldDeltaSeconds)))
    (:then_3
      (bind _asbp_player_controller (Utilities|Casting|CastToBP_PlayerController (Pawn|GetController)))
      (bind _output_get (Variables|Cursor|SetActorUnderCursor (.HitActor (Collision|BreakHitResult (.HitResult (Game|Player|GetHitResultUnderCursorbyChannel _asbp_player_controller "TraceTypeQuery1" true))))))
      (Utilities|IsValid _output_get
        (:Is%20Valid
          (Variables|Cursor|SetDistanceToActor (Math|Vector|VectorLength (- (Transformation|GetActorLocation (.HitActor (Collision|BreakHitResult (.HitResult (Game|Player|GetHitResultUnderCursorbyChannel _asbp_player_controller "TraceTypeQuery1" true))))) (Transformation|GetActorLocation)))))))))

(event Input|ActionEvents|InputActionSprintAction
  (params (Key :type Key%20Structure :default "None"))
  ;[1 1 1 1 23] СИГНАЛЫ С КЛАВИАТУРЫ
  ;;[1 1 1] Состояние бега
  (:Pressed
    (Variables|Default|SetSprintActivated true)
    (Utilities|FlowControl|Sequence :!label _label
      (:then_0
        (Class|TopDownShooterCharacter|ChangeMovementState))))
  (:Released
    (Variables|Default|SetSprintActivated false)
    (goto _label)))

(event Input|ActionEvents|InputActionWalkAction
  (params (Key :type Key%20Structure :default "None"))
  ;[1 1 1 1 23] СИГНАЛЫ С КЛАВИАТУРЫ
  ;;[1 1 1] Состояние бега
  (:Pressed
    (Variables|Default|SetWalkActivated true)
    (Class|TopDownShooterCharacter|ChangeMovementState :!label _label))
  (:Released
    (Variables|Default|SetWalkActivated false)
    (goto _label)))

(event Input|ActionEvents|InputActionInteraction
  (params (Key :type Key%20Structure :default "None"))
  (bind _actorundercursor (Variables|Cursor|GetActorUnderCursor))
  ;[1 1 1 1 23] СИГНАЛЫ С КЛАВИАТУРЫ
  ;;[1 1 1] Взаимодействие
  (:Pressed
    (Utilities|IsValid _actorundercursor
      (:Is%20Valid
        (if (and (<= (Variables|Cursor|GetDistanceToActor) (Variables|/Game/Blueprints/ActorComponents/InteractionSystem/BP_InteractionSystem.BP_InteractionSystem_C|GetInteractionDistance (Variables|Default|GetInteractionSystem))) (Utilities|DoesObjectImplementInterface _actorundercursor "/Game/Blueprints/Interfaces/BPI_Interactable.BPI_Interactable_C"))
          (Class|BPIInteractable|InteractwithTarget(Message) _actorundercursor self))))))

(event Input|AxisEvents|InputAxisCameraZoom
  (params (AxisValue :type Float%20%28single-precision%29))
  ;[1 1 1 1 23] СИГНАЛЫ С КЛАВИАТУРЫ
  ;;[1 1 1] Зум камеры
  (Camera|ModifyCameraDesiredHeight AxisValue (Variables|Camera|GetHeight%20Change%20Step)))

(event Input|MouseEvents|RightMouseButton
  (params (Key :type Key%20Structure :default "None"))
  ;[1 1 1 1 23] СИГНАЛЫ С КЛАВИАТУРЫ
  ;;[1 1 1] Состояние бега
  (:Pressed
    (Variables|Default|SetAimActivated true)
    (Class|TopDownShooterCharacter|ChangeMovementState :!label _label))
  (:Released
    (Variables|Default|SetAimActivated false)
    (goto _label)))

(event Input|MouseEvents|LeftMouseButton
  (params (Key :type Key%20Structure :default "None"))
  (bind _mesh (Variables|Character|GetMesh))
  ;[1 1 1 1 23] СИГНАЛЫ С КЛАВИАТУРЫ
  ;;[1 1 1] Анимация прицеливания
  (:Pressed
    (if (Variables|Default|GetAimActivated)
      (Animation|Montage|PlayMontage _mesh "/Game/Characters/Human/Animations/TDS_Fire_Rifle_Ironsights_Montage.TDS_Fire_Rifle_Ironsights_Montage" 1.0 0.0 "Default")
      (else
        (Animation|Montage|PlayMontage _mesh "/Game/Characters/Human/Animations/TDS_Fire_Rifle_Hip_Montage.TDS_Fire_Rifle_Hip_Montage" 1.0 0.0 "Default")))))

(fn ConstructionScript
  (bind _cameraboom (Variables|Default|GetCameraBoom))
  (Transformation|SetRelativeRotation _cameraboom (Variables|Camera|GetRotation) false false)
  (Variables|/Script/Engine.SpringArmComponent|SetCameraLagSpeed _cameraboom (Variables|Camera|GetSmoothness))
  (Variables|/Script/Engine.SpringArmComponent|SetbEnableCameraLag _cameraboom (Variables|Camera|GetSmoothMove)))

(fn SetupCameraDesiredHeight
  (Variables|Camera|SetDesired%20Height (Variables|/Script/Engine.SpringArmComponent|GetTargetArmLength (Variables|Default|GetCameraBoom))))

(fn ModifyCameraDesiredHeight
  (params (Direction :type Float%20%28single-precision%29) (Step :type Float%20%28single-precision%29))
  (bind _cameraboom (Variables|Default|GetCameraBoom))
  (LocalVariables|SetCamHeightStep Step)
  (Math|Float|CompareFloat Direction 0.0
    (:>
      (Math|Float|CompareFloat (+ (LocalVariables|GetCamHeightStep) (Variables|/Script/Engine.SpringArmComponent|GetTargetArmLength _cameraboom)) (Variables|Camera|GetMax%20Height)
        (:<
          (Variables|Camera|SetDesired%20Height (+ (LocalVariables|GetCamHeightStep) (Variables|/Script/Engine.SpringArmComponent|GetTargetArmLength _cameraboom))))))
    (:<
      (Math|Float|CompareFloat (- (Variables|/Script/Engine.SpringArmComponent|GetTargetArmLength _cameraboom) (LocalVariables|GetCamHeightStep)) (Variables|Camera|GetMin%20Height)
        (:>
          (Variables|Camera|SetDesired%20Height (- (Variables|/Script/Engine.SpringArmComponent|GetTargetArmLength _cameraboom) (LocalVariables|GetCamHeightStep))))))))

(fn InterpolateCamera
  (params (DeltaTime :type Float%20%28single-precision%29))
  (bind _desired_height (Variables|Camera|GetDesired%20Height))
  (if (!= (Variables|/Script/Engine.SpringArmComponent|GetTargetArmLength (Variables|Default|GetCameraBoom)) _desired_height)
    (Variables|/Script/Engine.SpringArmComponent|SetTargetArmLength (Variables|Default|GetCameraBoom) (Math|Interpolation|FInterpTo (Variables|/Script/Engine.SpringArmComponent|GetTargetArmLength (Variables|Default|GetCameraBoom)) _desired_height DeltaTime 5.0))))

(fn DoCameraShake
  (Camera|PlayWorldCameraShake "/Game/Blueprints/Game/BP_CameraShake.BP_CameraShake_C" (Transformation|GetWorldLocation (Variables|Default|GetTopDownCameraComponent)) 0.0 3e+01))

(fn DebugDrawInfo
  (bind _returnvalue (Transformation|GetVelocity))
  (bind _healthandstaminasystem (Variables|Components|GetHealthAndStaminaSystem))
  (bind _actorundercursor (Variables|Cursor|GetActorUnderCursor))
  (bind _returnvalue_2 (Components|GetOwner _actorundercursor))
  (if (Pawn|IsPlayerControlled)
    (Utilities|FlowControl|Sequence
      (:then_0
        (Development|PrintString (Utilities|String|Append "[BP_Player] Stamina: " (Utilities|String|ToString(Float) (Variables|/Game/Blueprints/ActorComponents/BP_HealthSystem.BP_HealthSystem_C|GetCurrentStamina _healthandstaminasystem))) true false "(R=0.000000,G=0.660000,B=1.000000,A=1.000000)" 0.0)
        (Development|PrintString (Utilities|String|Append "[BP_Player] Distance to Cursor Actor: " (Utilities|String|ToString(Float) (Variables|Cursor|GetDistanceToActor))) true false "(R=0.000000,G=0.660000,B=1.000000,A=1.000000)" 0.0)
        (Utilities|IsValid _actorundercursor
          (:Is%20Valid
            (Development|PrintString (Utilities|String|Append "[BP_Player]Cursor Actor Name: " (Utilities|String|SelectString (Utilities|GetDisplayName _actorundercursor) "None" (Utilities|IsValid _actorundercursor))) true false "(R=0.352837,G=1.000000,B=0.000000,A=1.000000)" 0.0)
            (Development|PrintString (Utilities|String|Append "[BP_Player]Cursor Actor Owner Name: " (Utilities|String|SelectString (Utilities|GetDisplayName _returnvalue_2) "None" (Utilities|IsValid _returnvalue_2))) true false "(R=0.352837,G=1.000000,B=0.000000,A=1.000000)" 0.0))))
      (:then_1
        (bind _value (Default|GetCurrentStaminaRegenDelay _healthandstaminasystem))
        (Development|PrintString (Utilities|String|Append "[BP_Player] Stamina Regen Delay: " (Utilities|String|ToString(Float) _value)) true false "(R=0.000000,G=0.660000,B=1.000000,A=1.000000)" 0.0))
      (:then_2
        (Development|PrintString (Utilities|String|Append "[BP_Player] Stamina Regen Rate: " (Utilities|String|ToString(Float) (Variables|/Game/Blueprints/ActorComponents/BP_HealthSystem.BP_HealthSystem_C|GetStaminaRegenRate _healthandstaminasystem))) true false "(R=0.000000,G=0.660000,B=1.000000,A=1.000000)" 0.0))
      (:then_3
        (Development|PrintString (Utilities|String|Append "[BP_Player] Velocity: " (Utilities|String|ToString(Float) (Math|Vector|VectorLength _returnvalue))) true false "(R=0.000000,G=0.660000,B=1.000000,A=1.000000)" 0.0))
      (:then_4
        (Development|PrintString (Utilities|String|Append "[BP_Player] Direction: " (Utilities|String|ToString(Float) (Class|AnimInstance|CalculateDirection (Components|SkeletalMesh|GetAnimInstance (Variables|Character|GetMesh)) _returnvalue (Transformation|GetActorRotation)))) true false "(R=0.000000,G=0.660000,B=1.000000,A=1.000000)" 0.0)))))

(fn UpdateStamina
  (Utilities|FlowControl|Sequence
    (:then_0
      ;[1 1 1] Отправить текущую стамину в С++
      (Variables|Default|SetCurrentStaminaCPP (Variables|/Game/Blueprints/ActorComponents/BP_HealthSystem.BP_HealthSystem_C|GetCurrentStamina (Variables|Components|GetHealthAndStaminaSystem))))
    (:then_1
      ;[1 1 1] Динамическое изменение настоящих затрат выносливости
      ; в зависимости от состояния передвижения
      (Default|SetStaminaConsumption (Variables|Components|GetHealthAndStaminaSystem) (Math|Float|SelectFloat (.SprintConsumption (Utilities|Struct|BreakCharacterStaminaInfo (Variables|Default|GetMovementStaminaConsumption))) 0.0 (Utilities|TDSPlayer:IsSprinting?))))))