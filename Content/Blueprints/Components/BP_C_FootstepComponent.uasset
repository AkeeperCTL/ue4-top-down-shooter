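; Footstep component that plays walk or run sounds at its location when DoFootstep is called with an animation name.
; A one-meter downward trace from the owner, with debug drawing, confirms ground.
; Substring matching of the animation name against two word sets sets the sound keyword, which selects an attenuated cue.
; The surface type switch has empty branches, so only Rubblestone cues play.
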(event Custom|Event%20Do%20Footstep
  (params (AnimationName :type String))
  (bind (_outhit _returnvalue) (|Трасировкалучавнизна1метр))
  (if _returnvalue
    (|Определениеключевогословадлязвука AnimationName)
    (switch Utilities|FlowControl|Switch|SwitchonEPhysicalSurface (Variables|/Script/PhysicsCore.PhysicalMaterial|GetSurfaceType (.PhysMat (Collision|BreakHitResult _outhit)))
      (:SurfaceType_Default
        _)
      (:SurfaceType1
        _))
    (|Проигрываниезвукаходьбы (Variables|Default|GetCurrentSoundKeyword))))

(event EventBeginPlay)

(event EventTick
  (params (DeltaSeconds :type Float%20%28single-precision%29)))

(fn AnimIsHaveWord
  (params (Words :type Array%20of%20Strings) (AnimationName :type String))
  (bind _array_element (Utilities|Array|ForEachLoopwithBreak Words :!label _label)
    (:LoopBody
      (if (Utilities|String|Contains AnimationName _array_element)
        (LocalVariables|SetLocalFindWord true)
        (goto _label Break)))
    (:Completed
      (return (LocalVariables|GetLocalFindWord)))))