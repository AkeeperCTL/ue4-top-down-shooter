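; Actor component that holds an actor's health and stamina, each with enable switches, maximums and optional regeneration.
; Setters update values and fire added, subtracted and zeroed dispatchers with a flag separating forced changes from damage or regeneration.
; Tick runs only stamina, applying a consumption rate and regenerating after a countdown that restarts whenever stamina drops.
; UpdateHealth offers health regeneration but is never called here and is marked untested, needing a rework like stamina's.
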(event Custom|OnStaminaSubtracted
  (params (Actor :type Actor%20Object%20Reference) (IsDamage :type Boolean)))

(event Custom|OnHealthZeroed
  (params (Actor :type Actor%20Object%20Reference)))

(event Custom|OnHealthAdded
  (params (Actor :type Actor%20Object%20Reference) (IsRegeneration :type Boolean)))

(event Custom|OnHealthSubtracted
  (params (Actor :type Actor%20Object%20Reference) (IsDamage :type Boolean)))

(event Custom|OnStaminaZeroed
  (params (Actor :type Actor%20Object%20Reference)))

(event Custom|OnStaminaAdded
  (params (Actor :type Actor%20Object%20Reference) (IsRegeneration :type Boolean)))

(event EventTick
  (params (DeltaSeconds :type Float%20%28single-precision%29))
  (Stamina|UpdateStamina))

(event EventBeginPlay
  (bind _maxhealth (Variables|Health|GetMaxHealth))
  (bind _maxstamina (Variables|Stamina|GetMaxStamina))
  (Utilities|FlowControl|Sequence
    (:then_0
      (Variables|Stamina|SetCurrentStaminaRegenStartDelay (Variables|Stamina|GetStaminaRegenStartDelay)))
    (:then_1
      (if (> (Variables|Health|GetCurrentHealth) _maxhealth)
        (Variables|Health|SetCurrentHealth _maxhealth)
        (if (> (Variables|Stamina|GetCurrentStamina) _maxstamina)
          (Variables|Stamina|SetCurrentStamina _maxstamina))))))

(fn SetCurrentHealth
  (params (value :type Float%20%28single-precision%29) (IsForced :type Boolean))
  (bind _returnvalue (Components|GetOwner))
  (bind _returnvalue_2 (not IsForced))
  (if (Variables|Health|GetEnableHealth)
    (if (>= value (Variables|Health|GetMaxHealth))
      (Variables|Health|SetCurrentHealth (Variables|Health|GetMaxHealth))
      (else
        (Variables|Health|SetCurrentHealth value)))
    (if (< value (Variables|Health|GetCurrentHealth))
      (CallFunction|OnHealthSubtracted _returnvalue _returnvalue_2)
      (else
        (CallFunction|OnHealthAdded _returnvalue _returnvalue_2)))
    (if (<= (Variables|Health|GetCurrentHealth) 0.0)
      (CallFunction|OnHealthZeroed (Components|GetOwner)))))

(fn SetMaxHealth
  (params (value :type Float%20%28single-precision%29))
  (if (Variables|Health|GetEnableHealth)
    (bind _output_get (Variables|Health|SetMaxHealth value))
    (if (> (Variables|Health|GetCurrentHealth) _output_get)
      (Health|SetCurrentHealth (Variables|Health|GetMaxHealth) true))))

(fn GetCurrentStaminaRegenDelay
  (return (Variables|Stamina|GetCurrentStaminaRegenStartDelay)))

(fn SetCurrentStamina
  (params (value :type Float%20%28single-precision%29) (IsForced :type Boolean))
  (bind _returnvalue (Components|GetOwner))
  (bind _returnvalue_2 (not IsForced))
  (LocalVariables|SetNewStamina (Math|Float|Clamp(Float) value 0.0 (Variables|Stamina|GetMaxStamina)))
  (if (Variables|Stamina|GetEnableStamina)
    (LocalVariables|SetSubtractingStamina (< (LocalVariables|GetNewStamina) (Variables|Stamina|GetCurrentStamina)))
    (Variables|Stamina|SetCurrentStamina (LocalVariables|GetNewStamina))
    (if (LocalVariables|GetSubtractingStamina)
      (CallFunction|OnStaminaSubtracted _returnvalue _returnvalue_2)
      (Variables|Stamina|SetCurrentStaminaRegenStartDelay (Variables|Stamina|GetStaminaRegenStartDelay)) ; -
      (else
        (CallFunction|OnStaminaAdded _returnvalue _returnvalue_2)))
    (if (<= (Variables|Stamina|GetCurrentStamina) 0.0)
      (CallFunction|OnStaminaZeroed (Components|GetOwner)))))

(fn SetMaxStamina
  (params (value :type Float%20%28single-precision%29))
  (if (Variables|Stamina|GetEnableStamina)
    (bind _output_get (Variables|Stamina|SetMaxStamina value))
    (if (> (Variables|Stamina|GetCurrentStamina) _output_get)
      (Stamina|SetCurrentStamina (Variables|Stamina|GetMaxStamina) true))))

(fn UpdateHealth
  (bind _maxhealth (Variables|Health|GetMaxHealth))
  (bind _currenthealth (Variables|Health|GetCurrentHealth))
  ;[1 1 1] НЕ ТЕСТИРОВАЛОСЬ, НАДО ПЕРЕДЕЛАТЬ!!! (КАК В СТАМИНЕ)
  (if (Variables|Health|GetEnableHealth)
    (if (Variables|Health|GetEnableHealthRegen)
      (if (< _currenthealth _maxhealth)
        (if (> (- (Utilities|Time|GetTimeSeconds) 1.0) (Variables|Health|GetHealthRegenStartDelay))
          (Health|SetCurrentHealth (+ _currenthealth (* (/ _maxhealth (Variables|Health|GetHealthRegenRate)) (Utilities|Time|GetWorldDeltaSeconds))) false))))))

(fn SetStaminaConsumption
  (params (Value :type Float%20%28single-precision%29))
  (Variables|Stamina|SetCurrentStaminaConsumptionValue Value))

(fn UpdateStamina
  (bind _returnvalue (Utilities|Time|GetWorldDeltaSeconds))
  (bind _currentstaminaconsumptionvalue (Variables|Stamina|GetCurrentStaminaConsumptionValue))
  (if (Variables|Stamina|GetEnableStamina)
    (if (Variables|Stamina|GetEnableStaminaRegen)
      ;[1 1 1] РАСХОД СТАМИНЫ С РЕГЕНЕРАЦИЕЙ
      (if (> (Variables|Stamina|GetCurrentStaminaRegenStartDelay) 0.0)
        (Variables|Stamina|SetCurrentStaminaRegenStartDelay (- (Variables|Stamina|GetCurrentStaminaRegenStartDelay) (Utilities|Time|GetWorldDeltaSeconds)))
        ;[1 1 1] РАСХОД СТАМИНЫ
        (if (> _currentstaminaconsumptionvalue 0.0) :!label _label
          (Stamina|SetCurrentStamina (- (Variables|Stamina|GetCurrentStamina) (* _currentstaminaconsumptionvalue (Utilities|Time|GetWorldDeltaSeconds))) false))
        (else
          (Stamina|SetCurrentStamina (- (+ (Variables|Stamina|GetCurrentStamina) (* (/ (Variables|Stamina|GetMaxStamina) (Variables|Stamina|GetStaminaRegenRate)) _returnvalue)) (* _returnvalue (Variables|Stamina|GetCurrentStaminaConsumptionValue))) false)))
      (else
        (goto _label)))))