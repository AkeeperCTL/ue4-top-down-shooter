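; Experimental arena template that procedurally builds a rectangular tiled room on BeginPlay, unless already generated.
; Child-actor floors fill the grid; the perimeter gets random wall meshes with indexed collision actors, leaving one gap in non-start rooms.
; Eligible slots may spawn doors instead, using a random stream weighted by the remaining door quota.
; The construction script and regeneration clear old pieces, sweeping owned leftover actors by class.
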(event EventBeginPlay
  (if (not (Variables|ArenaGeneration|GetIsGenerationComplete))
    (ArenaGeneration|GenerateNewArena)))

(event Collision|EventActorBeginOverlap
  (params (OtherActor :type Actor%20Object%20Reference)))

(event EventTick
  (params (DeltaSeconds :type Float%20%28single-precision%29)))

(fn ConstructionScript
  (ArenaGeneration|DestroyCurrentArena))

(fn CreateFloorCopies
  (params (TileX :type Integer) (TileY :type Integer) (TileStep :type Float%20%28single-precision%29))
  (for _index (range 0 TileX)
    (for _index_2 (range 0 TileY)
      (AddComponent|AddChildActorComponent false (Math|Transform|MakeTransform (Math|Vector|MakeVector (* _index TileStep) (* _index_2 TileStep) 0.0)))
      (Utilities|Array|Add (Variables|Walls&FloorCreation|GetSpawnedFloors) 0))))

(fn CreateWallCopies
  (params (TileX :type Integer) (Tile%20Y :type Integer) (Tile%20Step :type Float%20%28single-precision%29))
  (bind _wallsamplepoint (Variables|Default|GetWallSamplePoint))
  (bind _relativelocation (Variables|/Script/Engine.SceneComponent|GetRelativeLocation _wallsamplepoint))
  (LocalVariables|SetLocalTileX TileX)
  (bind _output_get (LocalVariables|SetLocalTileY Tile%20Y))
  (bind _output_get_2 (LocalVariables|SetLocalTileStep Tile%20Step))
  ;[1 1 1] НИЖНИЕ СТЕНЫ
  (for _index (range 0 _output_get)
    (if (or (Variables|ArenaGeneration|GetIsStartRoom) (!= _index 0))
      (CallFunction|DoororWall (== (Math|Integer|%(Integer) _index (Variables|ArenaGeneration|GetDoorDesiredIndex)) (Variables|ArenaGeneration|GetDoorDesiredRemainder)) (Math|Vector|MakeVector (.x _relativelocation) (* _index _output_get_2) (.z _relativelocation)) "0,90.000000, 0"))
    ;[1 1 1] ВЕРХНИЕ СТЕНЫ
    (CallFunction|DoororWall (== (Math|Integer|%(Integer) _index (Variables|ArenaGeneration|GetDoorDesiredIndex)) (Variables|ArenaGeneration|GetDoorDesiredRemainder)) (Math|Vector|MakeVector (+ (* (LocalVariables|GetLocalTileX) (LocalVariables|GetLocalTileStep)) (/ (LocalVariables|GetLocalTileStep) 2.0)) (* _index (LocalVariables|GetLocalTileStep)) (.z (Variables|/Script/Engine.SceneComponent|GetRelativeLocation (Variables|Default|GetWallSamplePoint)))) "0.0,-90.000000,0.0"))
  ;[1 1 1] СТЕНЫ СЛЕВА
  (for _index_2 (range 0 (LocalVariables|GetLocalTileX))
    (CallFunction|DoororWall (== (Math|Integer|%(Integer) _index_2 (Variables|ArenaGeneration|GetDoorDesiredIndex)) (Variables|ArenaGeneration|GetDoorDesiredRemainder)) (Math|Vector|MakeVector (* _index_2 (LocalVariables|GetLocalTileStep)) (- 0.0 (/ (LocalVariables|GetLocalTileStep) 2.0)) (.z (Variables|/Script/Engine.SceneComponent|GetRelativeLocation (Variables|Default|GetWallSamplePoint)))) "0.0,180.000000,0.000000")
    ;[1 1 1] СТЕНЫ СПРАВА
    (CallFunction|DoororWall (== (Math|Integer|%(Integer) _index_2 2) 1) (Math|Vector|MakeVector (* _index_2 (LocalVariables|GetLocalTileStep)) (+ (* (LocalVariables|GetLocalTileY) (LocalVariables|GetLocalTileStep)) (/ (LocalVariables|GetLocalTileStep) 2.0)) (.z (Variables|/Script/Engine.SceneComponent|GetRelativeLocation (Variables|Default|GetWallSamplePoint)))) "0, 0, 0")))

(fn DoororWall
  (params (CanBeDoor? :type Boolean) (RelativeTransform :type Vector) (RelativeRotation :type Rotator))
  (bind _returnvalue (Transformation|GetActorTransform))
  (bind _doordesiredcount (Variables|ArenaGeneration|GetDoorDesiredCount))
  (bind _returnvalue_2 (Math|Transform|TransformLocation _returnvalue RelativeTransform))
  (bind _returnvalue_3 (Math|Transform|TransformRotation _returnvalue RelativeRotation))
  (bind (_roll _pitch _yaw) (Math|Rotator|BreakRotator _returnvalue_3))
  (bind _returnvalue_4 (+ _yaw 9e+01))
  (bind _returnvalue_5 (Math|Rotator|MakeRotator _roll _pitch _returnvalue_4))
  (if (and CanBeDoor? (Class|KismetMathLibrary|RandomBoolwithWeightfromStream (/ (Math|Conversions|ToFloat(Integer) (- _doordesiredcount (Utilities|Array|Length (Variables|DoorCreation|GetSpawnedDoors)))) (Math|Conversions|ToFloat(Integer) _doordesiredcount)) (Variables|ArenaGeneration|GetRandomStreamVar)))
    ;[1 1 1] СОЗДАТЬ ДВЕРЬ
    (Game|SpawnActorfromClass (Variables|ArenaGeneration|GetUsedDoorClass) (Math|Transform|MakeTransform _returnvalue_2 _returnvalue_5 "1,1,1") "AlwaysSpawn" self 0)
    (Utilities|Array|Add (Variables|DoorCreation|GetSpawnedDoors) 0)
    (else
      ;[1 1 1] СОЗДАТЬ ОБЫЧНУЮ СТЕНУ
      (bind _returnvalue_6 (AddComponent|AddStaticMeshComponent false (Math|Transform|MakeTransform RelativeTransform RelativeRotation "1,1,1")))
      (Components|StaticMesh|SetStaticMesh _returnvalue_6 (.OutItem (Utilities|Array|Random (Variables|ArenaGeneration|GetUsedWallRandomMeshes))))
      (bind _returnvalue_7 (Utilities|Array|Add (Variables|Walls&FloorCreation|GetSpawnedWalls) _returnvalue_6))
      ;;[1 1 1] Создать номер стены
      (bind _returnvalue_8 (Game|SpawnActorfromClass "/Game/Blueprints/Environment/Arena/ArenaChilds/BP_ArenaWallCollision.BP_ArenaWallCollision_C" (Math|Transform|MakeTransform _returnvalue_2 _returnvalue_5 "1,1,1") "AlwaysSpawn" self _returnvalue_7 0 0))
      (Utilities|Array|AddUnique (Variables|Walls&FloorCreation|GetSpawnedWallCollisionIndexes) _returnvalue_8))))

(fn GenerateNewArena
  ;[1 1 1] ОЧИЩЕНИЕ ПОСТРОЕННЫХ КОМПОНЕНТОВ.
  ;
  ; КОГДА В РЕДАКТОРЕ ВЫЗЫВАЕШЬ ГЕНЕРАЦИЮ АРЕНЫ, ТО СТАРАЯ АРЕНА НЕ ИСЧЕЗАЕТ
  (ArenaGeneration|DestroyCurrentArena)
  (CallFunction|CreateFloorCopies (Variables|ArenaGeneration|GetArenaTilesX) (Variables|ArenaGeneration|GetArenaTilesY) (Variables|ArenaGeneration|GetArenaTilesStep))
  (CallFunction|CreateWallCopies (Variables|ArenaGeneration|GetArenaTilesX) (Variables|ArenaGeneration|GetArenaTilesY) (Variables|ArenaGeneration|GetArenaTilesStep))
  (Variables|ArenaGeneration|SetIsGenerationComplete true))

(fn DestroyCurrentArena
  (bind _spawnedwallcollisionindexes (Variables|Walls&FloorCreation|GetSpawnedWallCollisionIndexes))
  (bind _spawnedfloors (Variables|Walls&FloorCreation|GetSpawnedFloors))
  (bind _spawneddoors (Variables|DoorCreation|GetSpawnedDoors))
  (bind _spawnedwalls (Variables|Walls&FloorCreation|GetSpawnedWalls))
  ;[1 1 1] УНИЧТОЖЕНИЕ СТЕН
  (for _array_element _spawnedwalls
    (Utilities|IsValid _array_element
      (:Is%20Valid
        (Components|DestroyComponent _array_element))))
  (Utilities|Array|Clear _spawnedwalls)
  ;[1 1 1] УНИЧТОЖЕНИЕ НОМЕРАЦИИ СТЕН
  (for _array_element_2 _spawnedwallcollisionindexes
    (Utilities|IsValid _array_element_2
      (:Is%20Valid
        (Actor|DestroyActor _array_element_2))))
  (Utilities|Array|Clear _spawnedwallcollisionindexes)
  (|Дополнительноеудалениеоставшихсянумераций "/Game/Blueprints/Environment/Arena/ArenaChilds/BP_ArenaWallCollision.BP_ArenaWallCollision_C"
    (:Done
      ;[1 1 1] УНИЧТОЖЕНИЕ ПОЛА
      (for _array_element_3 _spawnedfloors
        (Utilities|IsValid _array_element_3
          (:Is%20Valid
            (Components|DestroyComponent _array_element_3))))
      (Utilities|Array|Clear _spawnedfloors)
      ;[1 1 1] УНИЧТОЖЕНИЕ ДВЕРЕЙ
      (for _array_element_4 _spawneddoors
        (Utilities|IsValid _array_element_4
          (:Is%20Valid
            (Actor|DestroyActor _array_element_4))))
      (Utilities|Array|Clear _spawneddoors)
      (|Дополнительноеудалениеоставшихсядверей (Variables|ArenaGeneration|GetUsedDoorClass)
        (:Done
          (Variables|ArenaGeneration|SetIsGenerationComplete false)
          (return))))))