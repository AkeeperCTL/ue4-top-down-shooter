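; Arena wall collision actor that carries an index, shows it on a text component and can be removed through interaction.
; The arena's generation event passes in the index and owning Arena, and the label refreshes then and in the construction script.
; Removal destroys the actor and reports its index back to the Arena.
; A debug function triggers the interaction; removal on door overlap exists but is disconnected.
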(event Custom|RemoveThis
  ;[1 1 1] Удаление
  (Actor|DestroyActor)
  (Class|BPIWallCollisionListener|OnWallCollisionDeleted(Message) (Variables|Default|GetArena) (Variables|Default|GetIndex)))

(event EventBeginPlay)

(event EventOnWallCollisionGenerated
  (params (Index :type Integer) (Arena :type BP%20Arena%201200%20Template%203%20Actual%20Object%20Reference))
  ;[1 1 1] Спавн коллизии по событию, вызванному в арене
  (Variables|Default|SetIndex Index)
  (Variables|Default|SetArena Arena)
  (CallFunction|UpdateIndexValue))

(event EventInteractwithTarget
  (params (Interaction-causing%20Actor :type Actor%20Object%20Reference))
  ;[1 1 1] Взаимодействие
  (Development|PrintString "Interact with wall number")
  (CallFunction|RemoveThis))

(event Collision|EventActorBeginOverlap
  (params (OtherActor :type Actor%20Object%20Reference))
  ;[1 1 1] Пересечение с дверью убирает стену
)

(fn ConstructionScript
  (CallFunction|UpdateIndexValue))

(fn UpdateIndexValue
  (Rendering|Components|TextRender|SetText (Variables|Default|GetIndexNumber) (Utilities|Text|ToText(Integer) (Variables|Default|GetIndex))))

(fn DebugDoInteract
  (Class|BPIInteractable|InteractwithTarget(Message) self))