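; Deprecated arena template actor that procedurally lays out a tiled floor and a row of walls in its construction script.
; CreateFloorInstances fills a grid of Floor mesh instances from the X and Y tile counts and a step spacing.
; Wall instances run along local X but use the Y tile count, a noted workaround for the wrongly rotated wall model.
; The event graph holds no logic.
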(event EventBeginPlay)

(event Collision|EventActorBeginOverlap
  (params (OtherActor :type Actor%20Object%20Reference)))

(event EventTick
  (params (DeltaSeconds :type Float%20%28single-precision%29)))

(fn ConstructionScript
  (CallFunction|CreateFloorInstances (Variables|Creation|GetArenaTilesX) (Variables|Creation|GetArenaTilesY) (Variables|Creation|GetStep))
  (for _index (range 0 (Variables|Creation|GetArenaTilesY))
    (Components|InstancedStaticMesh|AddInstance (Variables|Default|Getwall) (Math|Conversions|ToTransform(Vector) (Math|Vector|MakeVector (* _index (Variables|Creation|GetStep)) 0.0 0.0)))))

(fn CreateFloorInstances
  (params (TileX :type Integer) (TileY :type Integer) (TileStep :type Float%20%28single-precision%29))
  (for _index (range 0 TileX)
    (for _index_2 (range 0 TileY)
      (Components|InstancedStaticMesh|AddInstance (Variables|Default|Getfloor) (Math|Transform|MakeTransform (Math|Vector|MakeVector (* _index TileStep) (* _index_2 TileStep) 0.0))))))