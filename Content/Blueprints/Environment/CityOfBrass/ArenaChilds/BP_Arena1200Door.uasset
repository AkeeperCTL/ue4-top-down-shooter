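; Arena door that slides vertically on interaction and procedurally generates the next arena the first time it moves.
; Timelines lerp the mesh along Z while interaction is disabled; the construction script caches the closed position and previews the open state.
; On first use, a forward trace checks for existing arena walls, then spawns the owner's arena template with random tile size, passing on door and wall settings.
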(event Custom|SpawnNewArea
  (bind _door_direction (Variables|Default|GetDoor%20Direction))
  (bind _returnvalue (Transformation|GetWorldLocation _door_direction))
  ;[1 1 1] Создание следующей арены
  ;;[1 1 1] Проверка на существование созданной арены перед дверью
  (bind _outhit (Collision|LineTraceByChannel _returnvalue (+ _returnvalue (* (Math|Vector|GetForwardVector _door_direction) 30000)) "TraceTypeQuery1" false 0 "Persistent" true "(R=1.000000,G=0.000000,B=0.000000,A=1.000000)" "(R=0.000000,G=1.000000,B=0.000000,A=1.000000)" 555.0))
  (Utilities|Casting|CastToBP_ArenaWallCollision (.HitActor (Collision|BreakHitResult _outhit))
    (:CastFailed
      (if (Variables|NextArenaGeneration|GetCan%20Generate%20Next%20Arena?)
        (bind _asbp_arena_1200_template_3_actual (Utilities|Casting|CastToBP_Arena1200_Template3_Actual (Components|GetOwner))
          (:then
            (Game|SpawnActorfromClass "/Game/Blueprints/Environment/CityOfBrass/Arena/BP_Arena1200_Template3_Actual.BP_Arena1200_Template3_Actual_C" (Math|Transform|MakeTransform (+ (Transformation|GetActorLocation) (* (Transformation|GetActorForwardVector) 5.5e+02)) (Transformation|GetActorRotation) "1,1,1") "AlwaysSpawn" 0 (Variables|NextArenaGeneration|GetNext%20Arena%20Type) (Math|Random|RandomIntegerinRange 3 6) (Math|Random|RandomIntegerinRange 3 6) (Variables|NextArenaGeneration|GetDoor%20Desired%20Remainder) (Variables|NextArenaGeneration|GetDoor%20Desired%20Index) (Variables|NextArenaGeneration|GetDoor%20Count%20Info) (Variables|/Game/Blueprints/Environment/CityOfBrass/Arena/BP_Arena1200_Template3_Actual.BP_Arena1200_Template3_Actual_C|GetUsedWallCollisionClass _asbp_arena_1200_template_3_actual) (Utilities|GetClass self) 0))
          (:CastFailed
            (Development|PrintString "Door: Арена не определена")))
        (else
          (Development|PrintString "Door: Дверь не может дальше генерировать арену"))))))

(event Custom|OnStopPlayingAnimation
  (Utilities|FlowControl|Sequence
    (:then_0
      (Variables|/Game/Blueprints/ActorComponents/InteractionSystem/BP_InteractionSystem.BP_InteractionSystem_C|SetCanInteractWithOtherActors? (Variables|Default|GetInteractionSystem) true))))

(event Custom|OnStartPlayingAnimation
  (Utilities|FlowControl|Sequence ; 0) ЗАПРЕТИТЬ ВЗАИМОДЕЙСТВИЕ\n1) СОЗДАТЬ СЛЕДУЮЩУЮ АРЕНУ\n2) ПРОИГРАТЬ ЭФФЕКТ ПЫЛИ\n3) ПРОИГРАТЬ ЭФФЕКТ ТРЯСКИ КАМЕРЫ
    (:then_0
      (Variables|/Game/Blueprints/ActorComponents/InteractionSystem/BP_InteractionSystem.BP_InteractionSystem_C|SetCanInteractWithOtherActors? (Variables|Default|GetInteractionSystem) false))
    (:then_1
      (Utilities|FlowControl|DoOnce false
        (:Completed
          (CallFunction|SpawnNewArea))))))

(event EventInteractwithTarget
  (params (Interaction-causing%20Actor :type Actor%20Object%20Reference))
  (bind _door (Variables|Default|GetDoor))
  (bind _closedstaterelativelocation (Variables|DoorAnimation|GetClosedStateRelativeLocation))
  (bind _closedstaterelativelocation_2 (Variables|DoorAnimation|GetClosedStateRelativeLocation))
  (bind _interactionsystem (Variables|Default|GetInteractionSystem))
  (bind _is_locked (Variables|DoorState|GetIs%20Locked))
  (bind _caninteractwithotheractors_ (Variables|/Game/Blueprints/ActorComponents/InteractionSystem/BP_InteractionSystem.BP_InteractionSystem_C|GetCanInteractWithOtherActors? _interactionsystem))
  ;[1 1 1] ВЗАИМОДЕЙСТВИЕ
  (if (and _caninteractwithotheractors_ (not _is_locked))
    (if (Variables|DoorState|GetIs%20Opened)
      (Variables|DoorState|SetIs%20Opened false)
      (CallFunction|OnStartPlayingAnimation)
      ;;[1 1 1] АНИМАЦИЯ ЗАКРЫТИЯ
      (bind _alpha (Timeline|Close%20Animation PlayFromStart)
        (:Update
          (Transformation|SetRelativeLocation _door (Math|Vector|MakeVector (.x _closedstaterelativelocation) (.y _closedstaterelativelocation) (Math|Float|Lerp (+ (.z _closedstaterelativelocation) (Variables|DoorAnimation|GetZOffsetAnimation)) (.z (Variables|DoorAnimation|GetClosedStateRelativeLocation)) _alpha)) false false))
        (:Finished
          (CallFunction|OnStopPlayingAnimation)))
      (else
        (Variables|DoorState|SetIs%20Opened true)
        (CallFunction|OnStartPlayingAnimation)
        ;;[1 1 1] АНИМАЦИЯ ОТКРЫТИЯ
        (bind _alpha_2 (Timeline|Open%20Animation PlayFromStart)
          (:Update
            (Transformation|SetRelativeLocation _door (Math|Vector|MakeVector (.x _closedstaterelativelocation_2) (.y _closedstaterelativelocation_2) (Math|Float|Lerp (.z _closedstaterelativelocation_2) (+ (.z (Variables|DoorAnimation|GetClosedStateRelativeLocation)) (Variables|DoorAnimation|GetZOffsetAnimation)) _alpha_2)) false false))
          (:Finished
            (CallFunction|OnStopPlayingAnimation)))))
    (else
      (CallFunction|DebugPrintFailInteractionCause _caninteractwithotheractors_ _is_locked))))

(fn ConstructionScript
  (CallFunction|Open/CloseDooronConstruct))

(fn Open/CloseDooronConstruct
  (bind _door (Variables|Default|GetDoor))
  (Variables|DoorAnimation|SetClosedStateRelativeLocation (Variables|/Script/Engine.SceneComponent|GetRelativeLocation _door)) ; ПРИ СРАБАТЫВАНИИ СКРИПТА, ОТНОСИТЕЛЬНОЕ ПОЛОЖЕНИЕ СБРАСЫВАЕТСЯ НА ТО, \nКОТОРОЕ УКАЗАНО В VIEWPORT.\n\nСОХРАНЕНИЕ ПОЛОЖЕНИЯ ДВЕРИ В ЕЁ ЗАКРЫТОМ СОСТОЯНИИ.\nНУЖНО ДЛЯ ТОГО, ЧТОБЫ ВО ВРЕМЯ АНИМАЦИИ МОЖНО\nБЫЛО ВЕРНУТЬ ДВЕРЬ В ЗАКРЫТОЕ СОСТОЯНИЕ
  (if (Variables|DoorState|GetIs%20Opened)
    (Transformation|SetRelativeLocation _door (Math|Vector|MakeVector 0.0 0.0 (+ (.z (Variables|DoorAnimation|GetClosedStateRelativeLocation)) (Variables|DoorAnimation|GetZOffsetAnimation))) false false)
    (else
      (Transformation|SetRelativeLocation _door (Variables|DoorAnimation|GetClosedStateRelativeLocation) false false))))

(fn DebugPrintFailInteractionCause
  (params (Can%20Interact :type Boolean) (Is%20Locked :type Boolean))
  (bind _self self)
  (bind _returnvalue (Utilities|GetDisplayName _self))
  (if (Variables|DoorDebug|GetIs%20Debug%20Log%20Enabled)
    (Utilities|FlowControl|Sequence
      (:then_0
        (if (not Can%20Interact)
          (Development|PrintString (Utilities|String|Append _returnvalue "::Door can not to interact!") true true "(R=1.000000,G=0.024480,B=0.000000,A=1.000000)" 4.0)))
      (:then_1
        (if Is%20Locked
          (Development|PrintString (Utilities|String|Append _returnvalue "::Door is locked!") true true "(R=1.000000,G=0.024480,B=0.000000,A=1.000000)" 4.0))))))

(fn DebugInteract
  (CallFunction|InteractwithTarget))