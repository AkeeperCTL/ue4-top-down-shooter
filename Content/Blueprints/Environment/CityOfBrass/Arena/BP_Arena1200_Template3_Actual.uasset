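; Procedural arena actor that builds a tiled floor ringed by walls and doors at BeginPlay, adding a shop facing off the first door in start arenas.
; Floor tiles are mesh components mapped by grid coordinate; perimeter slots become door actors by stream-seeded weighted chance, otherwise random-mesh walls with indexed collision actors.
; Deleting a wall collision swap-removes its wall.
; Teardown clears everything, sweeping leftover owned doors and collisions by class.
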(event Custom|OnArenaGenerated
  (bind _spawneddoors (Variables|ArenaDoorGeneration|GetSpawnedDoors))
  (bind _output (Utilities|Array|Get(acopy) _spawneddoors))
  (bind _returnvalue (Transformation|GetActorRotation _output))
  ;[1 1 1] Событие после генерации арены
  (Variables|ArenaGeneration|SetIsGenerationComplete true)
  (switch Utilities|FlowControl|Switch|SwitchonBPE_ArenaTypes (Variables|ArenaGeneration|GetArenaType)
    (:NewEnumerator0
      (bind _floormesh (Floor|GetFloorCenterInstance))
      (bind _returnvalue_2 (Game|SpawnActorfromClass "/Game/Blueprints/Environment/CityOfBrass/ArenaOtherActors/BP_Shop.BP_Shop_C" (Math|Transform|MakeTransform (Transformation|GetWorldLocation _floormesh) (Math|Rotator|MakeRotator (.roll _returnvalue) (.pitch _returnvalue) (* (.yaw _returnvalue) -1.0))) "AlwaysSpawn" 0 0))
      (Variables|OtherActors|SetArenaShop _returnvalue_2))))

(event Custom|OnArenaDestroyed
  ;[1 1 1] Событие после уничтожения арены
  (Variables|ArenaGeneration|SetIsGenerationComplete false))

(event EventBeginPlay
  (if (not (Variables|ArenaGeneration|GetIsGenerationComplete))
    (ArenaGeneration|GenerateNewArena)))

(event Collision|EventActorBeginOverlap
  (params (OtherActor :type Actor%20Object%20Reference)))

(event EventTick
  (params (DeltaSeconds :type Float%20%28single-precision%29)))

(event EventOnWallCollisionDeleted
  (params (WallIndex :type Integer))
  (bind _spawnedwalls (Variables|Walls&FloorCreation|GetSpawnedWalls))
  (bind _returnvalue (Utilities|Array|LastIndex _spawnedwalls))
  ;[1 1 1] Событие при уничтожении коллизии стены
  (Components|DestroyComponent (Utilities|Array|Get(acopy) _spawnedwalls WallIndex))
  (Utilities|Array|SetArrayElem _spawnedwalls WallIndex (Utilities|Array|Get(acopy) _spawnedwalls _returnvalue) true)
  (Utilities|Array|RemoveIndex (Variables|Walls&FloorCreation|GetSpawnedWalls) _returnvalue))

(event EventDestroyed
  (ArenaGeneration|DestroyCurrentArena))

(fn ConstructionScript
  (ArenaGeneration|DestroyCurrentArena))

(fn CreateWallCopies
  (params (TileX :type Integer) (Tile%20Y :type Integer) (Tile%20Step :type Float%20%28single-precision%29))
  (bind _wallsamplepoint (Variables|Default|GetWallSamplePoint))
  (bind _relativelocation (Variables|/Script/Engine.SceneComponent|GetRelativeLocation _wallsamplepoint))
  (LocalVariables|SetLocalTileX (- TileX 1))
  (bind _output_get (LocalVariables|SetLocalTileY (- Tile%20Y 1)))
  (bind _output_get_2 (LocalVariables|SetLocalTileStep Tile%20Step))
  ;[1 1 1] НИЖНИЕ СТЕНЫ
  (for _index (range 0 _output_get)
    (if (or (Utilities|Enum|Equal(Enum) (Variables|ArenaGeneration|GetArenaType) "NewEnumerator0") (!= _index 0))
      (CreateMeshes|SpawnDoororWall (== (Math|Integer|%(Integer) _index (Variables|ArenaDoorGeneration|GetDoorDesiredIndex)) (Variables|ArenaDoorGeneration|GetDoorDesiredRemainder)) (Math|Vector|MakeVector (.x _relativelocation) (* _index _output_get_2) (.z _relativelocation)) "0,90.000000, 0" (.BottomCount (Utilities|Struct|BreakBPS_DoorCountInfo (Variables|ArenaDoorGeneration|GetDoorCountInfo)))))
    ;[1 1 1] ВЕРХНИЕ СТЕНЫ
    (CreateMeshes|SpawnDoororWall (== (Math|Integer|%(Integer) _index (Variables|ArenaDoorGeneration|GetDoorDesiredIndex)) (Variables|ArenaDoorGeneration|GetDoorDesiredRemainder)) (Math|Vector|MakeVector (+ (* (LocalVariables|GetLocalTileX) (LocalVariables|GetLocalTileStep)) (/ (LocalVariables|GetLocalTileStep) 2.0)) (* _index (LocalVariables|GetLocalTileStep)) (.z (Variables|/Script/Engine.SceneComponent|GetRelativeLocation (Variables|Default|GetWallSamplePoint)))) "0.0,-90.000000,0.0" (.TopCount (Utilities|Struct|BreakBPS_DoorCountInfo (Variables|ArenaDoorGeneration|GetDoorCountInfo)))))
  ;[1 1 1] СТЕНЫ СЛЕВА
  (for _index_2 (range 0 (LocalVariables|GetLocalTileX))
    (CreateMeshes|SpawnDoororWall (== (Math|Integer|%(Integer) _index_2 (Variables|ArenaDoorGeneration|GetDoorDesiredIndex)) (Variables|ArenaDoorGeneration|GetDoorDesiredRemainder)) (Math|Vector|MakeVector (* _index_2 (LocalVariables|GetLocalTileStep)) (- 0.0 (/ (LocalVariables|GetLocalTileStep) 2.0)) (.z (Variables|/Script/Engine.SceneComponent|GetRelativeLocation (Variables|Default|GetWallSamplePoint)))) "0.0,180.000000,0.000000" (.LeftCount (Utilities|Struct|BreakBPS_DoorCountInfo (Variables|ArenaDoorGeneration|GetDoorCountInfo))))
    ;[1 1 1] СТЕНЫ СПРАВА
    (CreateMeshes|SpawnDoororWall (== (Math|Integer|%(Integer) _index_2 (Variables|ArenaDoorGeneration|GetDoorDesiredIndex)) (Variables|ArenaDoorGeneration|GetDoorDesiredRemainder)) (Math|Vector|MakeVector (* _index_2 (LocalVariables|GetLocalTileStep)) (+ (* (LocalVariables|GetLocalTileY) (LocalVariables|GetLocalTileStep)) (/ (LocalVariables|GetLocalTileStep) 2.0)) (.z (Variables|/Script/Engine.SceneComponent|GetRelativeLocation (Variables|Default|GetWallSamplePoint)))) "0, 0, 0" (.RightCount (Utilities|Struct|BreakBPS_DoorCountInfo (Variables|ArenaDoorGeneration|GetDoorCountInfo))))))

(fn CreateFloorCopies
  (params (TileX :type Integer) (TileY :type Integer) (TileStep :type Float%20%28single-precision%29))
  (for _index (range 0 (- TileX 1))
    (for _index_2 (range 0 (- TileY 1))
      (bind _returnvalue (AddComponent|AddStaticMeshComponent false (Math|Transform|MakeTransform (Math|Vector|MakeVector (* _index TileStep) (* _index_2 TileStep) 0.0) "0, 0, 0" "1,1.000000,1")))
      (Utilities|Map|Add (Variables|Walls&FloorCreation|GetFloorMatrixOrderMap) (Math|Vector2D|MakeVector2D (+ (Math|Conversions|ToFloat(Integer) _index) 1.0) (+ (Math|Conversions|ToFloat(Integer) _index_2) 1.0)) _returnvalue))))

(fn SpawnDoororWall
  (params (CanBeDoor? :type Boolean) (RelativeTransform :type Vector) (RelativeRotation :type Rotator) (DesiredDoorCount :type Integer))
  (bind _returnvalue (Transformation|GetActorTransform))
  (bind _returnvalue_2 (Math|Transform|TransformLocation _returnvalue RelativeTransform))
  (bind _returnvalue_3 (Math|Transform|TransformRotation _returnvalue RelativeRotation))
  (bind (_roll _pitch _yaw) (Math|Rotator|BreakRotator _returnvalue_3))
  (bind _returnvalue_4 (+ _yaw 9e+01))
  (bind _returnvalue_5 (Math|Rotator|MakeRotator _roll _pitch _returnvalue_4))
  (bind _output_get (LocalVariables|SetLocal%20Door%20Count DesiredDoorCount))
  ;[1 1 1] Фикс предупреждения / на 0 при генерации арены
  (if (!= _output_get 0)
    (if (and CanBeDoor? (Class|KismetMathLibrary|RandomBoolwithWeightfromStream (/ (Math|Conversions|ToFloat(Integer) (- (LocalVariables|GetLocal%20Door%20Count) (Utilities|Array|Length (Variables|ArenaDoorGeneration|GetSpawnedDoors)))) (Math|Conversions|ToFloat(Integer) (LocalVariables|GetLocal%20Door%20Count))) (Variables|ArenaGeneration|GetRandomStreamVar)))
      ;[1 1 1] СОЗДАТЬ ДВЕРЬ
      (bind _returnvalue_6 (Game|SpawnActorfromClass (Variables|ArenaGeneration|GetUsedDoorClass) (Math|Transform|MakeTransform _returnvalue_2 _returnvalue_5 "1,1,1") "AlwaysSpawn" self 0))
      (Utilities|Array|Add (Variables|ArenaDoorGeneration|GetSpawnedDoors) _returnvalue_6)
      (else
        ;[1 1 1] СОЗДАТЬ ОБЫЧНУЮ СТЕНУ
        (bind _returnvalue_7 (AddComponent|AddStaticMeshComponent false (Math|Transform|MakeTransform RelativeTransform RelativeRotation "1,1,1") :!label _label))
        (Components|StaticMesh|SetStaticMesh _returnvalue_7 (.OutItem (Utilities|Array|Random (Variables|ArenaGeneration|GetUsedWallRandomMeshes))))
        (bind _returnvalue_8 (Utilities|Array|Add (Variables|Walls&FloorCreation|GetSpawnedWalls) _returnvalue_7))
        ;;[1 1 1] Создать номер стены
        (bind _returnvalue_9 (Game|SpawnActorfromClass (Variables|ArenaGeneration|GetUsedWallCollisionClass) (Math|Transform|MakeTransform _returnvalue_2 _returnvalue_5 "1,1,1") "AlwaysSpawn" self 0))
        (Class|BPIArenaListener|OnWallCollisionGenerated(Message) _returnvalue_9 _returnvalue_8 self)
        (Utilities|Array|AddUnique (Variables|Walls&FloorCreation|GetSpawnedWallCollisions) _returnvalue_9)))
    (else
      (goto _label))))

(fn GenerateNewArena
  ;[1 1 1] ОЧИЩЕНИЕ ПОСТРОЕННЫХ КОМПОНЕНТОВ.
  ;
  ; КОГДА В РЕДАКТОРЕ ВЫЗЫВАЕШЬ ГЕНЕРАЦИЮ АРЕНЫ, ТО СТАРАЯ АРЕНА НЕ ИСЧЕЗАЕТ
  (ArenaGeneration|DestroyCurrentArena)
  (CreateMeshes|CreateFloorCopies (Variables|ArenaGeneration|GetArenaTilesX) (Variables|ArenaGeneration|GetArenaTilesY) (Variables|ArenaGeneration|GetArenaTilesStep))
  (CreateMeshes|CreateWallCopies (Variables|ArenaGeneration|GetArenaTilesX) (Variables|ArenaGeneration|GetArenaTilesY) (Variables|ArenaGeneration|GetArenaTilesStep))
  (CallFunction|OnArenaGenerated))

(fn DestroyCurrentArena
  (bind _floormatrixordermap (Variables|Walls&FloorCreation|GetFloorMatrixOrderMap))
  (bind _arenashop (Variables|OtherActors|GetArenaShop))
  (bind _spawnedwallcollisions (Variables|Walls&FloorCreation|GetSpawnedWallCollisions))
  (bind _spawneddoors (Variables|ArenaDoorGeneration|GetSpawnedDoors))
  (bind _spawnedwalls (Variables|Walls&FloorCreation|GetSpawnedWalls))
  ;[1 1 1] УДАЛЕНИЕ ПРОЧИХ АКТЁРОВ
  (Utilities|IsValid _arenashop
    (:Is%20Valid
      (Actor|DestroyActor _arenashop))
    (:Is%20Not%20Valid
      _))
  ;[1 1 1] УНИЧТОЖЕНИЕ СТЕН
  (for _array_element _spawnedwalls
    (Utilities|IsValid _array_element
      (:Is%20Valid
        (Components|DestroyComponent _array_element))))
  (Utilities|Array|Clear _spawnedwalls)
  ;[1 1 1] УНИЧТОЖЕНИЕ НОМЕРАЦИИ СТЕН
  (for _array_element_2 _spawnedwallcollisions
    (Utilities|IsValid _array_element_2
      (:Is%20Valid
        (Actor|DestroyActor _array_element_2))))
  (Utilities|Array|Clear _spawnedwallcollisions)
  (|Дополнительноеудалениеоставшихсянумераций (Variables|ArenaGeneration|GetUsedWallCollisionClass)
    (:Done
      ;[1 1 1] УНИЧТОЖЕНИЕ ПОЛА
      (bind _values (Utilities|Map|Values _floormatrixordermap))
      (for _array_element_3 _values
        (Utilities|IsValid _array_element_3
          (:Is%20Valid
            (Components|DestroyComponent _array_element_3))))
      (Utilities|Map|Clear _floormatrixordermap)
      ;[1 1 1] УНИЧТОЖЕНИЕ ДВЕРЕЙ
      (for _array_element_4 _spawneddoors
        (Utilities|IsValid _array_element_4
          (:Is%20Valid
            (Actor|DestroyActor _array_element_4))))
      (Utilities|Array|Clear _spawneddoors)
      (|Дополнительноеудалениеоставшихсядверей (Variables|ArenaGeneration|GetUsedDoorClass)
        (:Done
          (CallFunction|OnArenaDestroyed)
          (return))))))

(fn GetFloorInstance
  (params (Vector :type Vector%202D%20Structure :default "(X=1.000000,Y=1.000000)"))
  (bind _floormatrixordermap (Variables|Walls&FloorCreation|GetFloorMatrixOrderMap))
  (bind (_value _returnvalue) (Utilities|Map|Find _floormatrixordermap Vector))
  (if _returnvalue
    (return _value)
    (else
      (Development|PrintString "Arena: Can't find the floor instance by input vector" true true "(R=1.000000,G=0.000000,B=0.000000,A=1.000000)" 5.0))))

(fn GetFloorCenterInstance
  (bind _floormesh (Floor|GetFloorInstance (Math|Vector2D|MakeVector2D (Math|Conversions|ToFloat(Integer) (Math|Float|Round (+ (/ (Math|Conversions|ToFloat(Integer) (Variables|ArenaGeneration|GetArenaTilesX)) 2.0) 0.1))) (Math|Conversions|ToFloat(Integer) (Math|Float|Round (+ (/ (Math|Conversions|ToFloat(Integer) (Variables|ArenaGeneration|GetArenaTilesY)) 2.0) 0.1))))))
  (return _floormesh))